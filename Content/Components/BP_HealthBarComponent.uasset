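; BP_HealthBarComponent is a component meant to link a health bar display to the main HUD, a slider, and front and rear progress bars.
; Individual Attach functions store each widget reference after a validity check, printing an error string on failure.
; InitHealthBarComponent assigns all four at once, though its slider and front bar checks each test the other's input.
; UpdateHP is an empty stub, so no health display logic exists yet.
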(fn `AttachFrontProgressBar`
  (params (FrontProgressBar :type "ProgressBar Object Reference"))
  (`/Engine/EditorBlueprintResources/StandardMacros.IsValid` FrontProgressBar
    (:`Is Valid`
      (set `self.FrontProgressBar_ObjRef` FrontProgressBar))
    (:`Is Not Valid`
      (`KismetSystemLibrary.PrintString` (`self.FrontHPProgressAssignToErrorStringW_0`) false true (struct :`R` 1.0 :`A` 1.0)))))

(fn `AttachHUD`
  (params (MainHUD :type "HUD Object Reference"))
  (`/Engine/EditorBlueprintResources/StandardMacros.IsValid` MainHUD
    (:`Is Valid`
      (set `self.MainHUD_ObjRef` MainHUD)
      (return))
    (:`Is Not Valid`
      (`KismetSystemLibrary.PrintString` (`self.MainHUDAssignToErrorStringW`) false true (struct :`R` 1.0 :`A` 1.0)))))

(fn `AttachProgressSlider`
  (params (SliderObjRef :type "Slider Object Reference"))
  (`/Engine/EditorBlueprintResources/StandardMacros.IsValid` SliderObjRef
    (:`Is Valid`
      (set `self.Slider_ObjRef` SliderObjRef))
    (:`Is Not Valid`
      (`KismetSystemLibrary.PrintString` (`self.SliderAssignToErrorStringW_0`) false true (struct :`R` 1.0 :`A` 1.0)))))

(fn `AttachRearProgressBar`
  (params (RearProgressBar :type "ProgressBar Object Reference"))
  (`/Engine/EditorBlueprintResources/StandardMacros.IsValid` RearProgressBar
    (:`Is Valid`
      (set `self.RearProgressBar_ObjRef` RearProgressBar))
    (:`Is Not Valid`
      (`KismetSystemLibrary.PrintString` (`self.RearHPProgressAssignToErrorStringW`) false true (struct :`R` 1.0 :`A` 1.0)))))

(fn `InitHealthBarComponent`
  (params (Slider_ObjRef :type "Slider Object Reference") (FrontProgressBar_ObjRef :type "ProgressBar Object Reference") (RearProgressBar_ObjRef :type "ProgressBar Object Reference") (MainHUD_ObjRef :type "HUD Object Reference"))
  (`|ExecutionSequence`
    (:`then_0`
      (`/Engine/EditorBlueprintResources/StandardMacros.IsValid` FrontProgressBar_ObjRef
        (:`Is Valid`
          (set `self.Slider_ObjRef` Slider_ObjRef))
        (:`Is Not Valid`
          (`KismetSystemLibrary.PrintString` (`self.SliderAssignToErrorStringW_0`)))))
    (:`then_1`
      (`/Engine/EditorBlueprintResources/StandardMacros.IsValid` Slider_ObjRef
        (:`Is Valid`
          (set `self.FrontProgressBar_ObjRef` FrontProgressBar_ObjRef))
        (:`Is Not Valid`
          (`KismetSystemLibrary.PrintString` (`self.FrontHPProgressAssignToErrorStringW_0`)))))
    (:`then_2`
      (`/Engine/EditorBlueprintResources/StandardMacros.IsValid` RearProgressBar_ObjRef
        (:`Is Valid`
          (set `self.RearProgressBar_ObjRef` RearProgressBar_ObjRef))
        (:`Is Not Valid`
          (`KismetSystemLibrary.PrintString` (`self.RearHPProgressAssignToErrorStringW`)))))
    (:`then_3`
      (`/Engine/EditorBlueprintResources/StandardMacros.IsValid` MainHUD_ObjRef
        (:`Is Valid`
          (set `self.MainHUD_ObjRef` MainHUD_ObjRef))
        (:`Is Not Valid`
          (`KismetSystemLibrary.PrintString` (`self.MainHUDAssignToErrorStringW`)))))))

(fn `UpdateHP`
  (params (NewHP_F :type "Float (double-precision)" :default 100.0) (CurrentHP_F :type "Float (double-precision)" :default 100.0) (MaxHP_F :type "Float (double-precision)" :default 100.0)))